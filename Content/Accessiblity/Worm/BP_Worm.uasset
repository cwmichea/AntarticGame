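; Worm actor that stays hidden, then pops up after a short random delay on BeginPlay.
; The PopUp timeline drives the skeletal mesh's relative height, enabling Tick when raised.
; PopDown disables Tick and reverses the timeline, destroying the actor when it finishes.
; Tick is empty: the rotation, debug cone and view-cone/distance player detection that would trigger PopDown are disconnected, so nothing here calls it.
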(event Custom|PopUpAnim
  (Development|SetHiddeninGame (Variables|Default|GetSkeletalMesh) false false)
  (bind (_direction _newtrack_0) (Timeline|PopUp PlayFromStart)
    (:Update
      (Transformation|SetRelativeLocation (Variables|Default|GetSkeletalMesh) (Math|Vector|MakeVector 0.0 0.0 (* _newtrack_0 2.5e+02)) false false))
    (:Finished
      (switch Utilities|FlowControl|Switch|SwitchonETimelineDirection _direction
        (:Forward
          (Actor|Tick|SetActorTickEnabled true))
        (:Backward
          (Actor|DestroyActor))))))

(event Custom|PopDown
  (Actor|Tick|SetActorTickEnabled false)
  (bind (_direction _newtrack_0) (Timeline|PopUp Reverse)
    (:Update
      (Transformation|SetRelativeLocation (Variables|Default|GetSkeletalMesh) (Math|Vector|MakeVector 0.0 0.0 (* _newtrack_0 2.5e+02)) false false))
    (:Finished
      (switch Utilities|FlowControl|Switch|SwitchonETimelineDirection _direction
        (:Forward
          (Actor|Tick|SetActorTickEnabled true))
        (:Backward
          (Actor|DestroyActor))))))

(event EventBeginPlay
  (Development|SetHiddeninGame (Variables|Default|GetSkeletalMesh) true false)
  (Actor|Tick|SetActorTickEnabled false)
  (Utilities|FlowControl|Delay (Math|Random|RandomFloatinRange 0.0 3.0))
  (CallFunction|PopUpAnim))

(event EventTick
  (params (DeltaSeconds :type Float%20%28single-precision%29)))

(fn ConstructionScript)

(fn DebugViz)