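; WormHunter runs the worm-hunting game's startup and holds its accessibility options.
; On BeginPlay it sets game-only input, reapplies sound and subtitle settings, and after a second spawns ten worms at random ground points found by downward traces.
; Option events store each value and push it to sound-mix overrides, subtitles, colour-vision correction, a camera-shake parameter collection, UI-scale listeners or BP_Chicken.
; At setup, sound on/off overrides follow and replace the saved volume levels.
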(event EventBeginPlay
  (Input|SetInputModeGameOnly (Game|GetPlayerController 0))
  (Utilities|FlowControl|Sequence
    (:then_0
      (Class|GameplayStatics|SetBaseSoundMix "/Game/Accessiblity/Audio/CustomMix.CustomMix"))
    (:then_1
      (Utilities|Time|SetTimerbyFunctionName 0 "Spawn Worm" 1.0))
    (:then_2
      (CallFunction|SetupOptions))))

(event Custom|ToggleAllSoundsEnabled
  (params (Enabled :type Boolean))
  ;[1 1 1] Toggle All Sounds Enabled/Disabled
  (bind _output_get (Variables|GameOptions|SetIsAllSoundsEnabled Enabled))
  (Audio|SetSoundMixClassOverride "/Game/Accessiblity/Audio/CustomMix.CustomMix" "/Game/Accessiblity/Audio/MASTER.MASTER" (Math|Float|SelectFloat 1.0 0.0 _output_get) 1.0 0.0 true))

(event Custom|ChangeAllSoundsLevel
  (params (Level :type Float%20%28single-precision%29))
  ;[1 1 1] Change All Sounds Level
  (bind _output_get (Variables|GameOptions|SetAllSoundsLevel Level))
  (Audio|SetSoundMixClassOverride "/Game/Accessiblity/Audio/CustomMix.CustomMix" "/Game/Accessiblity/Audio/MASTER.MASTER" _output_get 1.0 0.0 true))

(event Custom|ToggleHoldToRun
  (params (Enable :type Boolean))
  ;[1 1 1] Toggle Hold to Run
  (bind _output_get (Variables|GameOptions|SetIsToggleToRun Enable))
  (bind _asbp_chicken (Utilities|Casting|CastToBP_Chicken (Game|GetPlayerCharacter 0)))
  (Variables|/Game/Accessiblity/Blueprints/BP_Chicken.BP_Chicken_C|SetIsToggleRunp _asbp_chicken _output_get))

(event Custom|SetSubtitleSize
  (params (Size :type Integer))
  ;[1 1 1] Set Subtitle Size
  (bind _output_get (Variables|GameOptions|SetSubtitleSize Size))
  (bind _returnvalue (Actor|GetActorOfClass "/Game/Accessiblity/Blueprints/BP_AdvancedSubtitles.BP_AdvancedSubtitles_C"))
  (Default|ChangeSubtitleSize _returnvalue (Utilities|Select :Index _output_get :Option%200 24 :Option%201 32 :Option%202 64)))

(event Custom|ToggleSubtitles
  (params (Enabled :type Boolean))
  ;[1 1 1] Enable/Disable Subtitles
  (Variables|GameOptions|SetIsSubtitlesEnabled Enabled)
  (bind _returnvalue (Actor|GetActorOfClass "/Game/Accessiblity/Blueprints/BP_AdvancedSubtitles.BP_AdvancedSubtitles_C"))
  (Default|ToggleIsEnabled _returnvalue (Variables|GameOptions|GetIsSubtitlesEnabled)))

(event Custom|ToggleSoundEffectsEnabled
  (params (IsSoundEffectsEnabled :type Boolean))
  ;[1 1 1] Enable/Disable Sound Effects
  (bind _output_get (Variables|GameOptions|SetIsSoundEffectsEnabled IsSoundEffectsEnabled))
  (Audio|SetSoundMixClassOverride "/Game/Accessiblity/Audio/CustomMix.CustomMix" "/Game/Accessiblity/Audio/FX.FX" (Math|Float|SelectFloat 1.0 0.0 _output_get) 1.0 0.0 true))

(event Custom|ChangeSoundEffectsLevel
  (params (Level :type Float%20%28single-precision%29))
  ;[1 1 1] Change Sound Effects Level
  (bind _output_get (Variables|GameOptions|SetSoundEffectsLevel Level))
  (Audio|SetSoundMixClassOverride "/Game/Accessiblity/Audio/CustomMix.CustomMix" "/Game/Accessiblity/Audio/FX.FX" _output_get 1.0 0.0 true))

(event Custom|SetColorVisionDeficiencyType
  (params (ColorVisionDeficiencyType :type E_ColorDeficiencyTypes%20Enum :default "NewEnumerator0"))
  ;[1 1 1] Set the Color Deficiency Type with Correction
  (Variables|GameOptions|SetColorVisionDeficiencyType ColorVisionDeficiencyType)
  (Class|WidgetBlueprintLibrary|SetColorVisionDeficiencyType (Utilities|Select :Index (Math|Conversions|ToInteger(Byte) (Variables|GameOptions|GetColorVisionDeficiencyType)) :Option%200 "NormalVision" :Option%201 "Deuteranope" :Option%202 "Protanope" :Option%203 "Tritanope") 1.0 true))

(event Custom|ScaleUI
  (params (Percent :type Float%20%28single-precision%29))
  ;[1 1 1] Call Scale UI Event for all listeners
  (bind _output_get (Variables|GameOptions|SetUIScalePercent Percent))
  (Default|CallScaleUIEvent _output_get))

(event Custom|ToggleHighContrastMode
  (params (Enabled :type Boolean))
  ;[1 1 1] Toggle High Contrast Mode
  (Variables|GameOptions|SetIsHighContrastModeEnabled Enabled)
  (bind _asbp_chicken (Utilities|Casting|CastToBP_Chicken (Game|GetPlayerCharacter 0)))
  (Default|ToggleHighVis _asbp_chicken (Variables|GameOptions|GetIsHighContrastModeEnabled)))

(event Custom|ToggleScaleUIEnabled
  (params (Enabled :type Boolean))
  ;[1 1 1] Toggle Scale UI
  (bind _output_get (Variables|GameOptions|SetIsScaleUIEnabled Enabled))
  (if _output_get
    (CallFunction|ScaleUI (Variables|GameOptions|GetUIScalePercent))
    (else
      (Default|CallScaleUIEvent 1.0) ; We dont want to save this scale percent, just update the UI back to default for any listeners
    )))

(event Custom|ToggleSingleInputMode
  (params (Enable :type Boolean))
  ;[1 1 1] Toggle Single Input Mode on the Character
  (bind _output_get (Variables|GameOptions|SetIsSingleInputMode Enable))
  (bind _asbp_chicken (Utilities|Casting|CastToBP_Chicken (Game|GetPlayerCharacter 0)))
  (Variables|/Game/Accessiblity/Blueprints/BP_Chicken.BP_Chicken_C|SetAutoCam _asbp_chicken _output_get))

(event Custom|ToggleCameraShake
  (params (Enabled :type Boolean))
  ;[1 1 1] Toggle Camera Shake
  (bind _output_get (Variables|GameOptions|SetIsCameraShake Enabled))
  (Rendering|Material|SetScalarParameterValue "/Game/Accessiblity/Accessible/Accessibility.Accessibility" "ShakeScale" (Math|Conversions|ToFloat(Boolean) _output_get) :!class /Script/Engine.KismetMaterialLibrary))

(fn ConstructionScript)

(fn SpawnWorm
  (for _index (range 1 10)
    (Variables|Default|SetRemaining%20Worms _index)
    (bind _output_get (LocalVariables|SetNew%20Location (Math|Vector|MakeVector (Math|Random|RandomFloatinRange -2e+03 2e+03) (Math|Random|RandomFloatinRange -2e+03 2e+03) 4e+03)))
    (bind _outhit (Collision|LineTraceByChannel _output_get (- _output_get "0, 0,8000.000000") "TraceTypeQuery1" false 0 "None"))
    (Game|SpawnActorfromClass "/Game/Accessiblity/Worm/BP_Worm.BP_Worm_C" (Math|Transform|MakeTransform (.Location (Collision|BreakHitResult _outhit)) (Math|Rotator|MakeRotator 0.0 0.0 (Math|Random|RandomFloatinRange 0.0 3.6e+02)) "1,1,1") "Undefined" 0 0)))

(fn SetupOptions
  (Utilities|FlowControl|Sequence
    (:then_0
      (Audio|SetSoundMixClassOverride "/Game/Accessiblity/Audio/CustomMix.CustomMix" "/Game/Accessiblity/Audio/FX.FX" (Variables|GameOptions|GetSoundEffectsLevel) 1.0 0.0 true))
    (:then_1
      (Audio|SetSoundMixClassOverride "/Game/Accessiblity/Audio/CustomMix.CustomMix" "/Game/Accessiblity/Audio/MASTER.MASTER" (Variables|GameOptions|GetAllSoundsLevel) 1.0 0.0 true))
    (:then_2
      (Audio|SetSoundMixClassOverride "/Game/Accessiblity/Audio/CustomMix.CustomMix" "/Game/Accessiblity/Audio/FX.FX" (Math|Float|SelectFloat 1.0 0.0 (Variables|GameOptions|GetIsSoundEffectsEnabled)) 1.0 0.0 true))
    (:then_3
      (Audio|SetSoundMixClassOverride "/Game/Accessiblity/Audio/CustomMix.CustomMix" "/Game/Accessiblity/Audio/MASTER.MASTER" (Math|Float|SelectFloat 1.0 0.0 (Variables|GameOptions|GetIsAllSoundsEnabled)) 1.0 0.0 true))
    (:then_4
      (CallFunction|ToggleSubtitles (Variables|GameOptions|GetIsSubtitlesEnabled)))
    (:then_5
      (CallFunction|SetSubtitleSize (Variables|GameOptions|GetSubtitleSize)))))