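; Moving, rotating platform actor that travels between two configurable points.
; The construction script builds two relative InterpToMovement control points from Spot0 and Spot1 and sets the travel duration from Time.
; Tick runs through a 0.1-second Delay, so the actor yaws by Speed in periodic steps independent of the translation.
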(event EventBeginPlay)

(event Collision|EventActorBeginOverlap
  (params (OtherActor :type Actor%20Object%20Reference)))

(event EventTick
  (params (DeltaSeconds :type Float%20%28single-precision%29))
  (Utilities|FlowControl|Delay 0.1)
  (Transformation|AddActorLocalRotation (Math|Rotator|MakeRotator 0.0 0.0 (Variables|Default|GetSpeed)) false false))

(fn ConstructionScript
  (bind _interptomovement (Variables|Default|GetInterpToMovement))
  (Variables|/Script/Engine.InterpToMovementComponent|SetControlPoints _interptomovement (Utilities|Array|MakeArray (Utilities|Struct|MakeInterpControlPoint (Variables|Default|GetSpot0) true) (Utilities|Struct|MakeInterpControlPoint (Variables|Default|GetSpot1) true)))
  (Variables|/Script/Engine.InterpToMovementComponent|SetDuration _interptomovement (Variables|Default|Gettime)))