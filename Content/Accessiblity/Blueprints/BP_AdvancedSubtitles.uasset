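; Accessibility Blueprint that shows timed subtitles for a given audio asset through a UI_Subtitle widget created on BeginPlay.
; DisplaySubtitle starts at the first entry, and UpdateSubtitle chains timers, using each next entry's Time as its delay.
; The last line stays until StopSubtitle or HideSubtitle clears it.
; Disabling stops the current subtitle, but DisplaySubtitle does not check IsEnabled; text size changes pass to the widget.
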(event Custom|DisplaySubtitle
  (params (Audio :type Sound%20Wave%20Object%20Reference))
  ;[1 1 1] Start displaying our Subtitle based on the passed in Audio
  (Variables|Default|SetCurrentAudioToSubtitle Audio)
  (Variables|Default|SetCurrentIndex 0)
  (CallFunction|UpdateSubtitle))

(event Custom|UpdateSubtitle
  ;[1 1 1] Update our Subtitle to the next one in the Audio
  (Default|SetSubtitleText (Variables|Default|GetUISubtitleRef) (.text (Utilities|Array|Get(acopy) (Variables|/Script/Engine.SoundWave|GetSubtitles (Variables|Default|GetCurrentAudioToSubtitle)) (Variables|Default|GetCurrentIndex))))
  (Math|Integer|IncrementInt (Variables|Default|GetCurrentIndex)
    (:%20%20
      (if (not (> (Variables|Default|GetCurrentIndex) (Utilities|Array|LastIndex (Variables|/Script/Engine.SoundWave|GetSubtitles (Variables|Default|GetCurrentAudioToSubtitle)))))
        (bind _returnvalue (Utilities|Time|SetTimerbyFunctionName 0 "UpdateSubtitle" (.time (Utilities|Array|Get(acopy) (Variables|/Script/Engine.SoundWave|GetSubtitles (Variables|Default|GetCurrentAudioToSubtitle)) (Variables|Default|GetCurrentIndex)))))
        (Variables|Default|SetTimerHandle _returnvalue)))))

(event Custom|HideSubtitle
  ;[1 1 1] Hide Subtitle
  (Default|SetSubtitleText (Variables|Default|GetUISubtitleRef)))

(event Custom|ChangeSubtitleSize
  (params (Size :type Integer))
  (Default|UpdateSubtitleSize (Variables|Default|GetUISubtitleRef) Size))

(event Custom|StopSubtitle
  ;[1 1 1] Stop the Subtitle that is currently being processed and hide any displayed
  (Utilities|Time|ClearandInvalidateTimerbyHandle (Variables|Default|GetTimerHandle))
  (CallFunction|HideSubtitle))

(event Custom|ToggleIsEnabled
  (params (Enabled :type Boolean))
  ;[1 1 1] Toggle Enabled/Disabled
  (bind _output_get (Variables|Default|SetIsEnabled Enabled))
  (if (not _output_get)
    (CallFunction|StopSubtitle)))

(event EventBeginPlay
  ;[1 1 1] Create our Subtitle Widget and add it to our Viewport
  (bind _returnvalue (UserInterface|CreateWidget "/Game/Accessiblity/UI/UI_Subtitle.UI_Subtitle_C"))
  (bind _output_get (Variables|Default|SetUISubtitleRef _returnvalue))
  (UserInterface|Viewport|AddtoViewport _output_get 0))

(fn ConstructionScript)